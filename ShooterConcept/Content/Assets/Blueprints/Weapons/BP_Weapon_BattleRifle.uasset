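; Battle rifle weapon with active cooling, barrel swapping, reload, a charge-powered railgun mode and a stabilizer that holds fire until inaccuracy clears.
; WeaponFunction aims the model, retracts it near obstacles, fires projectiles and updates BP_UI_BR.
; Shots add heat, which slows accuracy recovery, while the spare barrel's heat converts into railgun charge.
; Tick continues cooling and charging while holstered, and dropping copies state to a BP_WeaponDrop_BR.
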(event `self.ReceiveBeginPlay`
  ;[1 1 1] Battle Rifle - Specific Mechanics
  (set `self.WeaponType` "NewEnumerator0"))

(event `self.Action2Pressed`
  (bind _ui_ref (`self.UI_Ref`))
  ;[1 1 1] Battle Rifle - Specific Mechanics
  ;;[1 1 1] Toggle Railgun
  (if (`self.Busy`)
    _
    (elif (`self.Toggle Rail`)
      (bind _output_get (set `self.Toggle Rail` false))
      (bind _asbp_ui_br (cast `/Game/Assets/Blueprints/UI/BP_UI_BR` _ui_ref))
      (`/Game/Assets/Blueprints/UI/BP_UI_BR.ToggleRail` _asbp_ui_br _output_get)
      (else
        (bind _output_get_2 (set `self.Toggle Rail` true))
        (bind _asbp_ui_br_2 (cast `/Game/Assets/Blueprints/UI/BP_UI_BR` _ui_ref))
        (`/Game/Assets/Blueprints/UI/BP_UI_BR.ToggleRail` _asbp_ui_br_2 _output_get_2)))))

(event `self.SecondaryActionPressed`
  ;[1 1 1] Battle Rifle - Specific Mechanics
  ;;[1 1 1] Active Cooling
  (if (not (`self.Busy`))
    (bind _output_get (set `self.Cooling State` true))
    (bind _output_get_2 (set `self.Busy` _output_get))
    (bind _asbp_ui_br (cast `/Game/Assets/Blueprints/UI/BP_UI_BR` (`self.UI_Ref`)))
    (`/Game/Assets/Blueprints/UI/BP_UI_BR.ToggleCooling` _asbp_ui_br _output_get_2)))

(event `self.SecondaryActionReleased`
  ;[1 1 1] Battle Rifle - Specific Mechanics
  ;;[1 1 1] Active Cooling
  (bind _output_get (set `self.Cooling State` false))
  (bind _output_get_2 (set `self.Busy` _output_get))
  (bind _asbp_ui_br (cast `/Game/Assets/Blueprints/UI/BP_UI_BR` (`self.UI_Ref`)))
  (`/Game/Assets/Blueprints/UI/BP_UI_BR.ToggleCooling` _asbp_ui_br _output_get_2))

(event `self.Action3Pressed`
  ;[1 1 1] Battle Rifle - Specific Mechanics
  ;;[1 1 1] Barrel Swap
  (if (not (`self.Busy`))
    (set `self.Changing Barrel` true)
    (bind _output_get (set `self.Busy` true))
    (bind _asbp_ui_br (cast `/Game/Assets/Blueprints/UI/BP_UI_BR` (`self.UI_Ref`)))
    (`/Game/Assets/Blueprints/UI/BP_UI_BR.SwapBarrel` _asbp_ui_br _output_get)
    (`KismetSystemLibrary.Delay` (`self.BarrelSwapTime`))
    (set `self.Tmp1` (`self.Heat Active`))
    (set `self.Heat Active` (`self.Heat Spare`))
    (set `self.Heat Spare` (`self.Tmp1`))
    (bind _output_get_2 (set `self.Changing Barrel` false))
    (bind _asbp_ui_br_2 (cast `/Game/Assets/Blueprints/UI/BP_UI_BR` (`self.UI_Ref`)))
    (`/Game/Assets/Blueprints/UI/BP_UI_BR.SwapBarrel` _asbp_ui_br_2 _output_get_2)
    (set `self.Busy` false)))

(event `self.Action1Pressed`
  (bind _ui_ref (`self.UI_Ref`))
  ;[1 1 1] Battle Rifle - Specific Mechanics
  ;;[1 1 1] Stabilizer
  (if (`self.Busy`)
    _
    (elif (`self.Toggle Stabilizer`)
      (bind _output_get (set `self.Toggle Stabilizer` false))
      (bind _asbp_ui_br (cast `/Game/Assets/Blueprints/UI/BP_UI_BR` _ui_ref))
      (`/Game/Assets/Blueprints/UI/BP_UI_BR.ToggleStab` _asbp_ui_br _output_get)
      (else
        (bind _output_get_2 (set `self.Toggle Stabilizer` true))
        (bind _asbp_ui_br_2 (cast `/Game/Assets/Blueprints/UI/BP_UI_BR` _ui_ref))
        (`/Game/Assets/Blueprints/UI/BP_UI_BR.ToggleStab` _asbp_ui_br_2 _output_get_2)))))

(event `self.MainActionPressed`
  ;[1 1 1] Battle Rifle - Specific Mechanics
  (set `self.Firing State` true))

(event `self.MainActionReleased`
  ;[1 1 1] Battle Rifle - Specific Mechanics
  (set `self.Firing State` false))

(event `self.WeaponFunction`
  (params (AimPoint :type "Vector Structure") (DoesAimPointExist :type Boolean) (CameraRotation :type "Rotator Structure") (`UI Ref` :type "UserWidget Object Reference"))
  (bind (_returnvalue_x _returnvalue_y _returnvalue_z) (`KismetMathLibrary.BreakVector` (`KismetMathLibrary.RandomUnitVector`)))
  (bind _inaccuracy_base_rate (`self.Inaccuracy Base Rate`))
  (bind _returnvalue (`SceneComponent.K2_GetComponentRotation` (`self.WeaponModel`)))
  (bind _returnvalue_2 (`SceneComponent.K2_GetComponentToWorld` (`self.ProjectileSpawnPoint`)))
  (bind _returnvalue_3 (+ (* _returnvalue_z (`self.Inaccuracy`)) (.yaw (.rotation _returnvalue_2))))
  (bind _returnvalue_4 (+ (.pitch (.rotation _returnvalue_2)) (* _returnvalue_y (`self.Inaccuracy`))))
  (bind (_returnvalue_roll _returnvalue_pitch _returnvalue_yaw) (`KismetMathLibrary.BreakRotator` (`KismetMathLibrary.RInterpTo` _returnvalue (`KismetMathLibrary.FindLookAtRotation` (`SceneComponent.K2_GetComponentLocation` (`self.WeaponModel`)) AimPoint) (`GameplayStatics.GetWorldDeltaSeconds`) (`self.Animation Speed`))))
  ;[1 1 1] Weapon Function
  ;;[1 1 1] Weapon Rotation
  (set `self.IsThereNoObstacle` (> (`KismetMathLibrary.VSize` (- (`SceneComponent.K2_GetComponentLocation` (`self.DefaultSceneRoot`)) AimPoint)) 70.0))
  (if DoesAimPointExist
    (if (`self.IsThereNoObstacle`)
      (`SceneComponent.K2_SetWorldRotation` (`self.WeaponModel`) (`KismetMathLibrary.MakeRotator` 0.0 _returnvalue_pitch _returnvalue_yaw) false false)
      (`SceneComponent.K2_SetRelativeLocation` (`self.WeaponModel`) (`KismetMathLibrary.VInterpTo` (`SceneComponent.RelativeLocation` (`self.WeaponModel`)) (0.0 0.0 0.0) (`GameplayStatics.GetWorldDeltaSeconds`) (`self.Animation Speed`)) false false :!label _label)
      (else
        (`SceneComponent.K2_SetWorldRotation` (`self.WeaponModel`) (`KismetMathLibrary.RInterpTo` _returnvalue (`KismetMathLibrary.MakeRotator` (.roll CameraRotation) (`KismetMathLibrary.FClamp` (+ (.pitch CameraRotation) 85.0) -85.0 85.0) (.yaw CameraRotation)) (`GameplayStatics.GetWorldDeltaSeconds`) (`self.Animation Speed`)) false false)
        (`SceneComponent.K2_SetRelativeLocation` (`self.WeaponModel`) (`KismetMathLibrary.VInterpTo` (`SceneComponent.RelativeLocation` (`self.WeaponModel`)) (-40.0 0.0 20.0) (`GameplayStatics.GetWorldDeltaSeconds`) (`self.Animation Speed`)) false false)))
    (else
      (`SceneComponent.K2_SetWorldRotation` (`self.WeaponModel`) (`KismetMathLibrary.RInterpTo` _returnvalue CameraRotation (`GameplayStatics.GetWorldDeltaSeconds`) (`self.Animation Speed`)) false false)
      (goto _label)))
  ;;[1 1 1] Cooling
  (if (not (`self.Changing Barrel`))
    ;;;[1 1 1] Spare Barrel Cooling
    (bind _output_get (set `self.Heat Spare` (`KismetMathLibrary.FClamp` (- (`self.Heat Spare`) (* (`self.Cooling Spare`) (`GameplayStatics.GetWorldDeltaSeconds`))) 0.0 100.0)))
    ;;;[1 1 1] Heat to Charge conversion
    (if (> _output_get 0.0)
      (set `self.Charge` (`KismetMathLibrary.FClamp` (+ (`self.Charge`) (* (`self.Heat Charge Conversion`) (`GameplayStatics.GetWorldDeltaSeconds`))) 0.0 (`self.ChargeMax`))))
    (set `self.Heat Active` (`KismetMathLibrary.FClamp` (- (- (`self.Heat Active`) (* (`self.Cooling Passive`) (`GameplayStatics.GetWorldDeltaSeconds`))) (* (* (`self.Cooling Active`) (`KismetMathLibrary.Conv_BoolToInt` (`self.Cooling State`))) (`GameplayStatics.GetWorldDeltaSeconds`))) 0.0 100.0)))
  ;;[1 1 1] Inaccuracy Calculation
  (set `self.Inaccuracy Rate` (`KismetMathLibrary.FClamp` (* (- _inaccuracy_base_rate (* (`self.Heat Active`) (`self.Heat Inaccuracy Rate`))) (`GameplayStatics.GetWorldDeltaSeconds`)) 0.0 _inaccuracy_base_rate))
  (set `self.Inaccuracy` (`KismetMathLibrary.FClamp` (- (`self.Inaccuracy`) (`self.Inaccuracy Rate`)) 0.0 4.0))
  ;;[1 1 1] UI Updates
  (bind _asbp_ui_br (cast `/Game/Assets/Blueprints/UI/BP_UI_BR` (`self.UI_Ref`))
    (:`then`
      (`/Game/Assets/Blueprints/UI/BP_UI_BR.UpdateHeat` _asbp_ui_br (`self.Heat Active`))
      (`/Game/Assets/Blueprints/UI/BP_UI_BR.UpdateAmmoRes` _asbp_ui_br (`self.Mags`))
      (`/Game/Assets/Blueprints/UI/BP_UI_BR.UpdateAmmoMag` _asbp_ui_br (`self.Ammo`))
      (`/Game/Assets/Blueprints/UI/BP_UI_BR.UpdateInaccuracy` _asbp_ui_br (`self.Inaccuracy`))
      (`/Game/Assets/Blueprints/UI/BP_UI_BR.BatteryCharge` _asbp_ui_br (`self.Charge`))
      (`/Game/Assets/Blueprints/UI/BP_UI_BR.UpdateHeatSpare` _asbp_ui_br (`self.Heat Spare`))
      (if (`self.IsActiveWeapon`)
        ;;[1 1 1] Firing
        ;;;[1 1 1] Can we fire the weapon?
        (if (and (`self.IsThereNoObstacle`) (and (not (`self.Busy`)) (and (not (`self.Cooling State`)) (and (`self.Firing State`) (and (`self.Can Fire`) (> (`self.Ammo`) 0))))))
          (if (`self.Toggle Stabilizer`)
            (if (<= (`self.Inaccuracy`) 0.0)
              (if (`self.Toggle Rail`) :!label _label_2
                ;;;[1 1 1] Charged Shot
                (if (> (`self.Charge`) (`self.Charge Per Shot`))
                  (`|SpawnActorFromClass` "/Game/Assets/Blueprints/BP_BulletCharged.BP_BulletCharged_C" (`KismetMathLibrary.MakeTransform` (.location _returnvalue_2) (`KismetMathLibrary.MakeRotator` (.roll (.rotation _returnvalue_2)) _returnvalue_4 _returnvalue_3)) "Undefined" "OverrideRootScale" null null)
                  (set `self.Can Fire` false)
                  (set `self.Ammo` (- (`self.Ammo`) 1))
                  (set `self.Heat Active` (`KismetMathLibrary.FClamp` (+ (`self.Heat Active`) (`self.Heat Per Shot Boosted`)) 0.0 100.0))
                  (set `self.Inaccuracy` (+ (`self.Inaccuracy`) (`self.Inaccuracy Per Shot Boosted`)))
                  (set `self.Charge` (- (`self.Charge`) (`self.Charge Per Shot`)))
                  (`KismetSystemLibrary.Delay` (`self.Fire Delay`))
                  (set `self.Can Fire` true))
                (else
                  ;;;[1 1 1] Regular Shot
                  (`|SpawnActorFromClass` "/Game/Assets/Blueprints/BP_Bullet.BP_Bullet_C" (`KismetMathLibrary.MakeTransform` (.location _returnvalue_2) (`KismetMathLibrary.MakeRotator` (.roll (.rotation _returnvalue_2)) _returnvalue_4 _returnvalue_3)) "Undefined" "OverrideRootScale" null null)
                  (set `self.Can Fire` false)
                  (set `self.Ammo` (- (`self.Ammo`) 1))
                  (set `self.Heat Active` (`KismetMathLibrary.FClamp` (+ (`self.Heat Active`) (`self.Heat Per Shot`)) 0.0 100.0))
                  (set `self.Inaccuracy` (+ (`self.Inaccuracy`) (`self.Inaccuracy Per Shot`)))
                  (`KismetSystemLibrary.Delay` (`self.Fire Delay`))
                  (set `self.Can Fire` true))))
            (else
              (goto _label_2))))))
    (:`CastFailed`
      (`KismetSystemLibrary.PrintString` "Hello"))))

(event `self.WeaponDrop`
  (params (`Drop Direction` :type "Vector Structure"))
  ;[1 1 1] Weapon Drop
  (bind _returnvalue (`|SpawnActorFromClass` "/Game/Assets/Blueprints/Weapons/WeaponDrops/BP_WeaponDrop_BR.BP_WeaponDrop_BR_C" (`SceneComponent.K2_GetComponentToWorld` (`self.WeaponModel`)) "Undefined" "OverrideRootScale" null null))
  (set `/Game/Assets/Blueprints/Weapons/WeaponDrops/BP_WeaponDrop_BR.Mags` (`self.Mags`) _returnvalue)
  (set `/Game/Assets/Blueprints/Weapons/WeaponDrops/BP_WeaponDrop_BR.Ammo` (`self.Ammo`) _returnvalue)
  (set `/Game/Assets/Blueprints/Weapons/WeaponDrops/BP_WeaponDrop_BR.Charge` (`self.Charge`) _returnvalue)
  (set `/Game/Assets/Blueprints/Weapons/WeaponDrops/BP_WeaponDrop_BR.Heat Active` (`self.Heat Active`) _returnvalue)
  (set `/Game/Assets/Blueprints/Weapons/WeaponDrops/BP_WeaponDrop_BR.Heat Spare` (`self.Heat Spare`) _returnvalue)
  (set `/Game/Assets/Blueprints/Weapons/WeaponDrops/BP_WeaponDrop_BR.Cooling Spare` (`self.Cooling Spare`) _returnvalue)
  (set `/Game/Assets/Blueprints/Weapons/WeaponDrops/BP_WeaponDrop_BR.Cooling Passive` (`self.Cooling Passive`) _returnvalue)
  (set `/Game/Assets/Blueprints/Weapons/WeaponDrops/BP_WeaponDrop_BR.Heat Charge Conversion` (`self.Heat Charge Conversion`) _returnvalue)
  (`/Game/Assets/Blueprints/Weapons/WeaponDrops/BP_WeaponDrop.WeaponDropped` _returnvalue `Drop Direction` (not (`self.IsThereNoObstacle`)))
  (`self.K2_DestroyActor`))

(event `self.WeaponSwitchTo`
  (params (Player :type "/Game/Assets/Blueprints/BP_PlayerCharacter Object Reference"))
  ;[1 1 1] Things done only when the weapon is switched to or off of
  (set `self.IsActiveWeapon` true)
  (set `self.UI_Ref` (`/Game/Assets/Blueprints/BP_PlayerCharacter.BR UI Ref` Player)))

(event `self.WeaponSwitchOff`
  (params (Player :type "/Game/Assets/Blueprints/BP_PlayerCharacter Object Reference"))
  ;[1 1 1] Things done only when the weapon is switched to or off of
  (set `self.IsActiveWeapon` false))

(event `self.ReceiveTick`
  (params (DeltaSeconds :type "Float (single-precision)"))
  ;[1 1 1] Allows the weapon to cool down while holstered
  (if (not (`self.IsActiveWeapon`))
    ;;[1 1 1] Spare Barrel Cooling
    (bind _output_get (set `self.Heat Spare` (`KismetMathLibrary.FClamp` (- (`self.Heat Spare`) (* (`self.Cooling Spare`) (`GameplayStatics.GetWorldDeltaSeconds`))) 0.0 100.0)))
    ;;[1 1 1] Heat to Charge conversion
    (if (> _output_get 0.0)
      (set `self.Charge` (`KismetMathLibrary.FClamp` (+ (`self.Charge`) (* (`self.Heat Charge Conversion`) (`GameplayStatics.GetWorldDeltaSeconds`))) 0.0 (`self.ChargeMax`))))
    (set `self.Heat Active` (`KismetMathLibrary.FClamp` (- (- (`self.Heat Active`) (* (`self.Cooling Passive`) (`GameplayStatics.GetWorldDeltaSeconds`))) (* (* (`self.Cooling Active`) (`KismetMathLibrary.Conv_BoolToInt` (`self.Cooling State`))) (`GameplayStatics.GetWorldDeltaSeconds`))) 0.0 100.0))))

(event `self.ReloadPressed`
  (bind _ui_ref (`self.UI_Ref`))
  ;[1 1 1] Reload
  (if (`self.Busy`)
    _
    (elif (> (`self.Mags`) 0)
      (bind _asbp_ui_br (cast `/Game/Assets/Blueprints/UI/BP_UI_BR` _ui_ref))
      (`/Game/Assets/Blueprints/UI/BP_UI_BR.Reload` _asbp_ui_br true)
      (set `self.Busy` true)
      (`KismetSystemLibrary.Delay` (`self.Reload Time`))
      (bind _asbp_ui_br_2 (cast `/Game/Assets/Blueprints/UI/BP_UI_BR` _ui_ref))
      (`/Game/Assets/Blueprints/UI/BP_UI_BR.Reload` _asbp_ui_br_2 false)
      (set `self.Ammo` (`self.Mag Size`))
      (set `self.Mags` (- (`self.Mags`) 1))
      (set `self.Busy` false))))

(fn `UserConstructionScript`
  (`parent.UserConstructionScript`))
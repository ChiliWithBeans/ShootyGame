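; Glaive melee weapon Blueprint that thrusts forward on the main action and damages enemies it overlaps.
; A timeline drives the thrust, with model collision and damage enabled only for its opening window.
; While idle, the model smoothly rotates toward the aim point or camera, raising and pulling back when an obstacle is close, which blocks attacks.
; Dropping spawns a pickup that inherits blade state and destroys the weapon.
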(event `self.MainActionPressed`
  ;[1 1 1] Attack animation
  (if (and (not (`self.Busy`)) (`self.IsThereNoObstacle`))
    (set `self.Busy` true)
    ;;[1 1 1] Damage can only be dealt during the first 0.12 seconds of the attack animation
    (set `self.EnableDamage` true)
    (`PrimitiveComponent.SetCollisionEnabled` (`self.WeaponModel`) "QueryOnly")
    (bind (_direction _forward_movement) (`Timeline|Attack Animation` :!via `PlayFromStart`)
      (:`Update`
        (`SceneComponent.K2_SetRelativeLocation` (`self.WeaponModel`) (`KismetMathLibrary.MakeVector` (* _forward_movement 200.0)) false false))
      (:`Finished`
        (set `self.Busy` false))
      (:`Damage`
        (set `self.EnableDamage` false)
        (`PrimitiveComponent.SetCollisionEnabled` (`self.WeaponModel`) "NoCollision")))))

(event `self.ReceiveActorBeginOverlap`
  (params (OtherActor :type "Actor Object Reference"))
  ;[1 1 1] Deals damage upon overlapping with enemy
  (if (`self.EnableDamage`)
    (bind _asbp_enemy (cast `/Game/Assets/Blueprints/Enemies/BP_Enemy` OtherActor))
    (`/Game/Assets/Blueprints/Enemies/BP_Enemy.Take Damage` _asbp_enemy 100.0)))

(event `self.ReloadPressed`)

(event `self.WeaponDrop`
  (params (`Drop Direction` :type "Vector Structure"))
  ;[1 1 1] Weapon drop
  (bind _returnvalue (`|SpawnActorFromClass` "/Game/Assets/Blueprints/Weapons/WeaponDrops/BP_WeaponDrop_Glaive.BP_WeaponDrop_Glaive_C" (`SceneComponent.K2_GetComponentToWorld` (`self.WeaponModel`)) "Undefined" "OverrideRootScale" null null))
  (set `/Game/Assets/Blueprints/Weapons/WeaponDrops/BP_WeaponDrop_Glaive.Blades` (`self.Blades`) _returnvalue)
  (set `/Game/Assets/Blueprints/Weapons/WeaponDrops/BP_WeaponDrop_Glaive.Blade Integrity` (`self.Blade Integrity`) _returnvalue)
  (`/Game/Assets/Blueprints/Weapons/WeaponDrops/BP_WeaponDrop.WeaponDropped` _returnvalue `Drop Direction` false)
  (`self.K2_DestroyActor`))

(event `self.WeaponSwitchTo`
  (params (Player :type "/Game/Assets/Blueprints/BP_PlayerCharacter Object Reference"))
  ;[1 1 1] Used when weapon is switched to or off of
  (set `self.IsActiveWeapon` true)
  (set `self.UI_Ref` (`/Game/Assets/Blueprints/BP_PlayerCharacter.BR UI Ref` Player)))

(event `self.ReceiveBeginPlay`
  ;[1 1 1] No idea how to set this otherwise
  (`PrimitiveComponent.SetCollisionEnabled` (`self.WeaponModel`) "NoCollision"))

(event `self.WeaponSwitchOff`
  (params (Player :type "/Game/Assets/Blueprints/BP_PlayerCharacter Object Reference"))
  ;[1 1 1] Used when weapon is switched to or off of
  (set `self.IsActiveWeapon` false))

(event `self.WeaponFunction`
  (params (AimPoint :type "Vector Structure") (DoesAimPointExist :type Boolean) (CameraRotation :type "Rotator Structure") (`UI Ref` :type "UserWidget Object Reference"))
  (bind _returnvalue (`SceneComponent.K2_GetComponentRotation` (`self.WeaponModel`)))
  (bind (_returnvalue_roll _returnvalue_pitch _returnvalue_yaw) (`KismetMathLibrary.BreakRotator` (`KismetMathLibrary.RInterpTo` _returnvalue (`KismetMathLibrary.FindLookAtRotation` (`SceneComponent.K2_GetComponentLocation` (`self.WeaponModel`)) AimPoint) (`GameplayStatics.GetWorldDeltaSeconds`) (`self.Animation Speed`))))
  ;[1 1 1] Weapon Rotation
  (if (not (`self.Busy`))
    (set `self.IsThereNoObstacle` (> (`KismetMathLibrary.VSize` (- (`SceneComponent.K2_GetComponentLocation` (`self.DefaultSceneRoot`)) AimPoint)) 200.0))
    (if DoesAimPointExist
      (if (`self.IsThereNoObstacle`)
        (`SceneComponent.K2_SetWorldRotation` (`self.WeaponModel`) (`KismetMathLibrary.MakeRotator` 0.0 _returnvalue_pitch _returnvalue_yaw) false false)
        (`SceneComponent.K2_SetRelativeLocation` (`self.WeaponModel`) (`KismetMathLibrary.VInterpTo` (`SceneComponent.RelativeLocation` (`self.WeaponModel`)) (0.0 0.0 0.0) (`GameplayStatics.GetWorldDeltaSeconds`) (`self.Animation Speed`)) false false :!label _label)
        (else
          (`SceneComponent.K2_SetWorldRotation` (`self.WeaponModel`) (`KismetMathLibrary.RInterpTo` _returnvalue (`KismetMathLibrary.MakeRotator` (.roll CameraRotation) (`KismetMathLibrary.FClamp` (+ (.pitch CameraRotation) 85.0) -85.0 85.0) (.yaw CameraRotation)) (`GameplayStatics.GetWorldDeltaSeconds`) (`self.Animation Speed`)) false false)
          (`SceneComponent.K2_SetRelativeLocation` (`self.WeaponModel`) (`KismetMathLibrary.VInterpTo` (`SceneComponent.RelativeLocation` (`self.WeaponModel`)) (-40.0 0.0 20.0) (`GameplayStatics.GetWorldDeltaSeconds`) (`self.Animation Speed`)) false false)))
      (else
        (`SceneComponent.K2_SetWorldRotation` (`self.WeaponModel`) (`KismetMathLibrary.RInterpTo` _returnvalue CameraRotation (`GameplayStatics.GetWorldDeltaSeconds`) (`self.Animation Speed`)) false false)
        (goto _label)))))

(fn `UserConstructionScript`
  (`parent.UserConstructionScript`))
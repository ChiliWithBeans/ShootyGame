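; Dropped-weapon actor for the BR weapon, holding its magazines, ammo, charge and barrel heat until a player picks it up.
; Tick keeps cooling the active and spare barrels, converting spare-barrel heat into charge while any remains.
; Drops flagged as retracted add linear velocity and random spin to the physics mesh.
; Pickup passes the stored state to the player and destroys the actor; the overlap ammo-pickup handler only casts.
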(event `self.ReceiveTick`
  (params (DeltaSeconds :type "Float (single-precision)"))
  ;[1 1 1] Spare Barrel Cooling
  (bind _output_get (set `self.Heat Spare` (`KismetMathLibrary.FClamp` (- (`self.Heat Spare`) (* (`self.Cooling Spare`) (`GameplayStatics.GetWorldDeltaSeconds`))) 0.0 100.0)))
  ;[1 1 1] Heat to Charge conversion
  (if (> _output_get 0.0)
    (set `self.Charge` (`KismetMathLibrary.FClamp` (+ (`self.Charge`) (* (`self.Heat Charge Conversion`) (`GameplayStatics.GetWorldDeltaSeconds`))) 0.0 100.0)))
  (set `self.Heat Active` (`KismetMathLibrary.FClamp` (- (- (`self.Heat Active`) (* (`self.Cooling Passive`) (`GameplayStatics.GetWorldDeltaSeconds`))) 0.0) 0.0 100.0)))

(event `self.ReceiveBeginPlay`
  (set `self.WeaponType` "NewEnumerator0"))

(event `self.WeaponDropped`
  (params (`Drop Direction` :type "Vector Structure") (IsWeaponRetracted :type Boolean))
  (bind _mesh (`self.mesh`))
  ;[1 1 1] Sets velocity after being dropped, same for all weapons
  (if IsWeaponRetracted
    (`PrimitiveComponent.SetPhysicsLinearVelocity` _mesh `Drop Direction` true "None")
    (`PrimitiveComponent.SetAllPhysicsAngularVelocityInDegrees` _mesh (`KismetMathLibrary.MakeVector` (`KismetMathLibrary.RandomFloatInRange` -100.0 100.0) (`KismetMathLibrary.RandomFloatInRange` -100.0 100.0) (`KismetMathLibrary.RandomFloatInRange` -100.0 100.0)) true)))

(event `self.WeaponPickup`
  (params (Player :type "/Game/Assets/Blueprints/BP_PlayerCharacter Object Reference"))
  ;[1 1 1] Weapon Pickup
  (`/Game/Assets/Blueprints/BP_PlayerCharacter.WeaponPickupBR` Player (`self.Mags`) (`self.Ammo`) (`self.Charge`) (`self.Heat Active`) (`self.Heat Spare`))
  (`self.K2_DestroyActor`))

(event `self.ReceiveActorBeginOverlap`
  (params (OtherActor :type "Actor Object Reference"))
  ;[1 1 1] Makes the weapon act as an ammo pickup if you already have it on you
  (cast `/Game/Assets/Blueprints/BP_PlayerCharacter` OtherActor))

(fn `UserConstructionScript`
  (`parent.UserConstructionScript`))
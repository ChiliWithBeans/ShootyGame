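; Glaive weapon drop: the physical pickup actor for the Glaive, built on a parent Blueprint and tagged with its weapon type on BeginPlay.
; On pickup it hands its Blades and BladeIntegrity state to the player's WeaponPickupGlaive, then destroys itself.
; When dropped in a retracted state, it adds the drop direction to the mesh's physics velocity along with a random spin.
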(event `self.ReceiveBeginPlay`
  (set `self.WeaponType` "NewEnumerator2"))

(event `self.WeaponPickup`
  (params (Player :type "/Game/Assets/Blueprints/BP_PlayerCharacter Object Reference"))
  (`/Game/Assets/Blueprints/BP_PlayerCharacter.WeaponPickupGlaive` Player (`self.Blades`) (`self.Blade Integrity`))
  (`self.K2_DestroyActor`))

(event `self.WeaponDropped`
  (params (`Drop Direction` :type "Vector Structure") (IsWeaponRetracted :type Boolean))
  (bind _mesh (`self.mesh`))
  ;[1 1 1] Sets velocity after being dropped, same for all weapons
  (if IsWeaponRetracted
    (`PrimitiveComponent.SetPhysicsLinearVelocity` _mesh `Drop Direction` true "None")
    (`PrimitiveComponent.SetAllPhysicsAngularVelocityInDegrees` _mesh (`KismetMathLibrary.MakeVector` (`KismetMathLibrary.RandomFloatInRange` -100.0 100.0) (`KismetMathLibrary.RandomFloatInRange` -100.0 100.0) (`KismetMathLibrary.RandomFloatInRange` -100.0 100.0)) true)))

(fn `UserConstructionScript`
  (`parent.UserConstructionScript`))
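; Battle rifle weapon with reload, toggleable railgun coils and stabilizer, active cooling and barrel change.
; An externally called WeaponFunction interpolates aim, retracts near obstacles, updates the UI, cools both barrels and fires.
; Heat slows accuracy recovery, spare-barrel heat recharges the battery for charged shots, and the stabilizer holds fire until inaccuracy clears.
; Barrel change only sets busy flags; its delayed heat-swap logic is disconnected.
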(event `Reload`
  ;[1 1 1] Gun Mechanics
  ;;[1 1 1] Reload
  (if (`self.BR Busy`)
    _
    (elif (> (`self.BR Mags`) 0)
      (`/Game/Assets/Blueprints/UI/BP_UI_BR.Reload` (`self.UI_Ref`) true)
      (set `self.BR Busy` true)
      (`KismetSystemLibrary.Delay` (`self.BR Reload Time`))
      (`/Game/Assets/Blueprints/UI/BP_UI_BR.Reload` (`self.UI_Ref`) false)
      (set `self.BR Ammo` (`self.BR Mag Size`))
      (set `self.BR Mags` (- (`self.BR Mags`) 1))
      (set `self.BR Busy` false))))

(event `StartFiring`
  ;[1 1 1] Gun Mechanics
  ;;[1 1 1] Fire Weapon
  (set `self.BR Firing State` true))

(event `Railgun`
  (bind _ui_ref (`self.UI_Ref`))
  ;[1 1 1] Gun Mechanics
  ;;[1 1 1] Toggle Railgun Coils
  (if (`self.BR Busy`)
    _
    (elif (`self.BR Toggle Coils`)
      (bind _output_get (set `self.BR Toggle Coils` false))
      (`/Game/Assets/Blueprints/UI/BP_UI_BR.ToggleRail` _ui_ref _output_get)
      (else
        (bind _output_get_2 (set `self.BR Toggle Coils` true))
        (`/Game/Assets/Blueprints/UI/BP_UI_BR.ToggleRail` _ui_ref _output_get_2)))))

(event `ActiveCoolingStart`
  ;[1 1 1] Gun Mechanics
  ;;[1 1 1] Active Cooling
  (if (not (`self.BR Busy`))
    (set `self.BR Cooling State` true)
    (bind _output_get (set `self.BR Busy` true))
    (`/Game/Assets/Blueprints/UI/BP_UI_BR.ToggleCooling` (`self.UI_Ref`) _output_get)))

(event `StopFiring`
  ;[1 1 1] Gun Mechanics
  ;;[1 1 1] Fire Weapon
  (set `self.BR Firing State` false))

(event `ActiveCoolingStop`
  ;[1 1 1] Gun Mechanics
  ;;[1 1 1] Active Cooling
  (set `self.BR Cooling State` false)
  (bind _output_get (set `self.BR Busy` false))
  (`/Game/Assets/Blueprints/UI/BP_UI_BR.ToggleCooling` (`self.UI_Ref`) _output_get))

(event `BarrelChange`
  ;[1 1 1] Gun Mechanics
  ;;[1 1 1] Barrel Change
  (if (not (`self.BR Busy`))
    (set `self.BR Changing Barrel` true)
    (set `self.BR Busy` true)))

(event `Stabilizer`
  (bind _ui_ref (`self.UI_Ref`))
  ;[1 1 1] Gun Mechanics
  ;;[1 1 1] Stabilizer
  (if (`self.BR Busy`)
    _
    (elif (`self.BR Toggle Stabilizer`)
      (bind _output_get (set `self.BR Toggle Stabilizer` false))
      (`/Game/Assets/Blueprints/UI/BP_UI_BR.ToggleStab` _ui_ref _output_get)
      (else
        (bind _output_get_2 (set `self.BR Toggle Stabilizer` true))
        (`/Game/Assets/Blueprints/UI/BP_UI_BR.ToggleStab` _ui_ref _output_get_2)))))

(event `WeaponFunction`
  (params (AimPoint :type "Vector Structure") (DoesAimPointExist :type Boolean) (CameraRotation :type "Rotator Structure") (`UI Ref` :type "/Game/Assets/Blueprints/UI/BP_UI_BR Object Reference"))
  (bind (_returnvalue_x _returnvalue_y _returnvalue_z) (`KismetMathLibrary.BreakVector` (`KismetMathLibrary.RandomUnitVector`)))
  (bind _br_inaccuracy_base_rate (`self.BR Inaccuracy Base Rate`))
  (bind _returnvalue (`SceneComponent.K2_GetComponentRotation` (`self.simpleGun_Rifle1`)))
  (bind _returnvalue_2 (`SceneComponent.K2_GetComponentToWorld` (`self.ProjectileSpawnPoint`)))
  (bind _returnvalue_3 (+ (* _returnvalue_z (`self.BR Inaccuracy`)) (.yaw (.rotation _returnvalue_2))))
  (bind _returnvalue_4 (+ (.pitch (.rotation _returnvalue_2)) (* _returnvalue_y (`self.BR Inaccuracy`))))
  (bind (_returnvalue_roll _returnvalue_pitch _returnvalue_yaw) (`KismetMathLibrary.BreakRotator` (`KismetMathLibrary.RInterpTo` _returnvalue (`KismetMathLibrary.FindLookAtRotation` (`SceneComponent.K2_GetComponentLocation` (`self.simpleGun_Rifle1`)) AimPoint) (`GameplayStatics.GetWorldDeltaSeconds`) (`self.Animation Speed`))))
  ;[1 1 1] Weapon Function
  ;;[1 1 1] Weapon Rotation
  (set `self.IsThereNoObstacle` (> (`KismetMathLibrary.VSize` (- (`SceneComponent.K2_GetComponentLocation` (`self.DefaultSceneRoot`)) AimPoint)) 70.0))
  (if DoesAimPointExist
    (if (`self.IsThereNoObstacle`)
      (`SceneComponent.K2_SetWorldRotation` (`self.simpleGun_Rifle1`) (`KismetMathLibrary.MakeRotator` 0.0 _returnvalue_pitch _returnvalue_yaw) false false)
      (else
        (`SceneComponent.K2_SetWorldRotation` (`self.simpleGun_Rifle1`) (`KismetMathLibrary.RInterpTo` _returnvalue (`KismetMathLibrary.MakeRotator` (.roll CameraRotation) (`KismetMathLibrary.FClamp` (+ (.pitch CameraRotation) 85.0) -85.0 85.0) (.yaw CameraRotation)) (`GameplayStatics.GetWorldDeltaSeconds`) (`self.Animation Speed`)) false false)))
    (else
      (`SceneComponent.K2_SetWorldRotation` (`self.simpleGun_Rifle1`) (`KismetMathLibrary.RInterpTo` _returnvalue CameraRotation (`GameplayStatics.GetWorldDeltaSeconds`) (`self.Animation Speed`)) false false)))
  (if (`self.IsThereNoObstacle`)
    (`SceneComponent.K2_SetRelativeLocation` (`self.simpleGun_Rifle1`) (`KismetMathLibrary.VInterpTo` (`SceneComponent.RelativeLocation` (`self.simpleGun_Rifle1`)) (0.0 0.0 0.0) (`GameplayStatics.GetWorldDeltaSeconds`) (`self.Animation Speed`)) false false)
    (else
      (`SceneComponent.K2_SetRelativeLocation` (`self.simpleGun_Rifle1`) (`KismetMathLibrary.VInterpTo` (`SceneComponent.RelativeLocation` (`self.simpleGun_Rifle1`)) (-40.0 0.0 20.0) (`GameplayStatics.GetWorldDeltaSeconds`) (`self.Animation Speed`)) false false)))
  ;;[1 1 1] UI Updates
  (set `self.UI_Ref` `UI Ref`)
  (`/Game/Assets/Blueprints/UI/BP_UI_BR.UpdateHeat` (`self.UI_Ref`) (`self.BR Heat Active`))
  (`/Game/Assets/Blueprints/UI/BP_UI_BR.UpdateAmmoRes` (`self.UI_Ref`) (`self.BR Mags`))
  (`/Game/Assets/Blueprints/UI/BP_UI_BR.UpdateAmmoMag` (`self.UI_Ref`) (`self.BR Ammo`))
  (`/Game/Assets/Blueprints/UI/BP_UI_BR.UpdateInaccuracy` (`self.UI_Ref`) (`self.BR Inaccuracy`))
  (`/Game/Assets/Blueprints/UI/BP_UI_BR.BatteryCharge` (`self.UI_Ref`) (`self.BR Charge`))
  (`/Game/Assets/Blueprints/UI/BP_UI_BR.UpdateHeatSpare` (`self.UI_Ref`) (`self.BR Heat Spare`))
  ;;[1 1 1] Cooling
  (if (not (`self.BR Changing Barrel`))
    ;;;[1 1 1] Spare Barrel Cooling
    (bind _output_get (set `self.BR Heat Spare` (`KismetMathLibrary.FClamp` (- (`self.BR Heat Spare`) (* (`self.BR Cooling Spare`) (`GameplayStatics.GetWorldDeltaSeconds`))) 0.0 100.0)))
    ;;;[1 1 1] Heat to Charge conversion
    (if (> _output_get 0.0)
      (set `self.BR Charge` (`KismetMathLibrary.FClamp` (+ (`self.BR Charge`) (* (`self.BR Heat Charge Conversion`) (`GameplayStatics.GetWorldDeltaSeconds`))) 0.0 100.0)))
    (set `self.BR Heat Active` (`KismetMathLibrary.FClamp` (- (- (`self.BR Heat Active`) (* (`self.BR Cooling Passive`) (`GameplayStatics.GetWorldDeltaSeconds`))) (* (* (`self.BR Cooling Active`) (`KismetMathLibrary.Conv_BoolToInt` (`self.BR Cooling State`))) (`GameplayStatics.GetWorldDeltaSeconds`))) 0.0 100.0)))
  ;;[1 1 1] Inaccuracy Calculation
  (set `self.BR Inaccuracy Rate` (`KismetMathLibrary.FClamp` (* (- _br_inaccuracy_base_rate (* (`self.BR Heat Active`) (`self.BR Heat Inaccuracy Rate`))) (`GameplayStatics.GetWorldDeltaSeconds`)) 0.0 _br_inaccuracy_base_rate))
  (set `self.BR Inaccuracy` (`KismetMathLibrary.FClamp` (- (`self.BR Inaccuracy`) (`self.BR Inaccuracy Rate`)) 0.0 4.0))
  ;;[1 1 1] Firing
  ;;;[1 1 1] Can we fire the weapon?
  (if (and (`self.IsThereNoObstacle`) (and (not (`self.BR Busy`)) (and (not (`self.BR Cooling State`)) (and (`self.BR Firing State`) (and (`self.BR Can Fire`) (> (`self.BR Ammo`) 0))))))
    (if (`self.BR Toggle Stabilizer`)
      (if (<= (`self.BR Inaccuracy`) 0.0)
        (if (`self.BR Toggle Coils`) :!label _label
          ;;;[1 1 1] Charged Shot
          (if (> (`self.BR Charge`) (`self.BR Charge Per Shot`))
            (`|SpawnActorFromClass` "/Game/Assets/Blueprints/BP_BulletCharged.BP_BulletCharged_C" (`KismetMathLibrary.MakeTransform` (.location _returnvalue_2) (`KismetMathLibrary.MakeRotator` (.roll (.rotation _returnvalue_2)) _returnvalue_4 _returnvalue_3)) "Undefined" "OverrideRootScale" null null)
            (set `self.BR Can Fire` false)
            (set `self.BR Ammo` (- (`self.BR Ammo`) 1))
            (set `self.BR Heat Active` (`KismetMathLibrary.FClamp` (+ (`self.BR Heat Active`) (`self.BR Heat Shot Boosted`)) 0.0 100.0))
            (set `self.BR Inaccuracy` (+ (`self.BR Inaccuracy`) (`self.BR Inaccuracy Shot Charged`)))
            (set `self.BR Charge` (- (`self.BR Charge`) (`self.BR Charge Per Shot`)))
            (`KismetSystemLibrary.Delay` (`self.BR Fire Delay`))
            (set `self.BR Can Fire` true))
          (else
            ;;;[1 1 1] Regular Shot
            (`|SpawnActorFromClass` "/Game/Assets/Blueprints/BP_Bullet.BP_Bullet_C" (`KismetMathLibrary.MakeTransform` (.location _returnvalue_2) (`KismetMathLibrary.MakeRotator` (.roll (.rotation _returnvalue_2)) _returnvalue_4 _returnvalue_3)) "Undefined" "OverrideRootScale" null null)
            (set `self.BR Can Fire` false)
            (set `self.BR Ammo` (- (`self.BR Ammo`) 1))
            (set `self.BR Heat Active` (`KismetMathLibrary.FClamp` (+ (`self.BR Heat Active`) (`self.BR Heat Shot`)) 0.0 100.0))
            (set `self.BR Inaccuracy` (+ (`self.BR Inaccuracy`) (`self.BR Inaccuracy Shot`)))
            (`KismetSystemLibrary.Delay` (`self.BR Fire Delay`))
            (set `self.BR Can Fire` true))))
      (else
        (goto _label)))))

(event `OnPickedUp`
  (params (Magazines :type Integer) (Ammo :type Integer) (Charge :type "Float (double-precision)") (`Heat Active` :type "Float (double-precision)") (`Heat Spare` :type "Float (double-precision)"))
  (set `self.BR Mags` Magazines)
  (set `self.BR Ammo` Ammo)
  (set `self.BR Charge` Charge)
  (set `self.BR Heat Active` `Heat Active`)
  (set `self.BR Heat Spare` `Heat Spare`))

(fn `UserConstructionScript`)
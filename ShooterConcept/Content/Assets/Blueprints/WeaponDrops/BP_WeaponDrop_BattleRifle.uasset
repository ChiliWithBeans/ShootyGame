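; Dropped battle rifle pickup that carries the weapon's magazines, ammo, charge and heat state.
; WeaponDropped copies those stats and, unless the weapon is retracted, throws the physics mesh along the drop direction with random spin.
; While it lies in the world, Tick cools active and spare-barrel heat and builds charge while spare heat remains.
; WeaponPickup passes the updated stats to the player and destroys the actor.
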(event `self.ReceiveTick`
  (params (DeltaSeconds :type "Float (single-precision)"))
  ;[1 1 1] Spare Barrel Cooling
  (bind _output_get (set `self.Heat Spare` (`KismetMathLibrary.FClamp` (- (`self.Heat Spare`) (* (`self.Cooling Spare`) (`GameplayStatics.GetWorldDeltaSeconds`))) 0.0 100.0)))
  ;[1 1 1] Heat to Charge conversion
  (if (> _output_get 0.0)
    (set `self.Charge` (`KismetMathLibrary.FClamp` (+ (`self.Charge`) (* (`self.Heat Charge Conversion`) (`GameplayStatics.GetWorldDeltaSeconds`))) 0.0 100.0)))
  (set `self.Heat Active` (`KismetMathLibrary.FClamp` (- (- (`self.Heat Active`) (* (`self.Cooling Passive`) (`GameplayStatics.GetWorldDeltaSeconds`))) 0.0) 0.0 100.0)))

(event `WeaponDropped`
  (params (Magazines :type Integer) (Ammo :type Integer) (Charge :type "Float (double-precision)") (`Heat Active` :type "Float (double-precision)") (`Heat Spare` :type "Float (double-precision)") (`Cooling Spare` :type "Float (double-precision)") (`Cooling Passive` :type "Float (double-precision)") (`Heat Charge Conversion` :type "Float (double-precision)") (`Drop Direction` :type "Vector Structure") (IsWeaponRetracted :type Boolean))
  (bind _simplegun_rifle (`self.simpleGun_Rifle`))
  ;[1 1 1] Replicates stats of held weapon when dropped and applies momentum + random rotation
  (set `self.Magazines` Magazines)
  (set `self.Ammo` Ammo)
  (set `self.Charge` Charge)
  (set `self.Heat Active` `Heat Active`)
  (set `self.Heat Spare` `Heat Spare`)
  (set `self.Cooling Spare` `Cooling Spare`)
  (set `self.Cooling Passive` `Cooling Passive`)
  (set `self.Heat Charge Conversion` `Heat Charge Conversion`)
  (if (not IsWeaponRetracted)
    (`PrimitiveComponent.SetPhysicsLinearVelocity` _simplegun_rifle (* (`KismetMathLibrary.MakeVector` `Drop Direction_X` `Drop Direction_Y` 1.0) (`self.DropSpeed`)) true "None")
    (`PrimitiveComponent.SetAllPhysicsAngularVelocityInDegrees` _simplegun_rifle (`KismetMathLibrary.MakeVector` (`KismetMathLibrary.RandomFloatInRange` -100.0 100.0) (`KismetMathLibrary.RandomFloatInRange` -100.0 100.0) (`KismetMathLibrary.RandomFloatInRange` -100.0 100.0)) false)))

(event `WeaponPickup`
  (params (Player :type "/Game/Assets/Blueprints/BP_PlayerCharacter Object Reference"))
  ;[1 1 1] Weapon Pickup
  (`/Game/Assets/Blueprints/BP_PlayerCharacter.WeaponPickupBR` Player (`self.Magazines`) (`self.Ammo`) (`self.Charge`) (`self.Heat Active`) (`self.Heat Spare`))
  (`self.K2_DestroyActor`))

(fn `UserConstructionScript`)
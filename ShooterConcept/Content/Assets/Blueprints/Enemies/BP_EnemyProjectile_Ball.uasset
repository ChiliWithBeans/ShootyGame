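; Enemy ball projectile that damages the player on overlap.
; OnSpawn scales the actor's current velocity by the passed Speed, adds random spread on each axis to the ProjectileMovement velocity, then destroys the actor after its Lifetime.
; Overlapping the player calls HealthChange with Damage and leaves the ball alive, while overlapping any other actor destroys it.
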(event `OnSpawn`
  (params (Speed :type "Float (double-precision)"))
  (bind _spread (`self.Spread`))
  (bind (_returnvalue_x _returnvalue_y _returnvalue_z) (`KismetMathLibrary.BreakVector` (* (`self.GetVelocity`) Speed)))
  (bind _returnvalue (* _spread -1.0))
  (set `MovementComponent.Velocity` (`KismetMathLibrary.MakeVector` (+ (`KismetMathLibrary.RandomFloatInRange` _returnvalue _spread) _returnvalue_x) (+ (`KismetMathLibrary.RandomFloatInRange` _returnvalue _spread) _returnvalue_y) (+ (`KismetMathLibrary.RandomFloatInRange` _returnvalue _spread) _returnvalue_z)) (`self.ProjectileMovement`))
  (`KismetSystemLibrary.Delay` (`self.Lifetime`))
  (`self.K2_DestroyActor`))

(event `self.ReceiveActorBeginOverlap`
  (params (OtherActor :type "Actor Object Reference"))
  (bind _asbp_player_character (cast `/Game/Assets/Blueprints/BP_PlayerCharacter` OtherActor)
    (:`then`
      (`/Game/Assets/Blueprints/BP_PlayerCharacter.HealthChange` _asbp_player_character self 2 (`self.Damage`) false))
    (:`CastFailed`
      (`self.K2_DestroyActor`))))

(fn `UserConstructionScript`
  (`parent.UserConstructionScript`))
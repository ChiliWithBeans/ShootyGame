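; Plasma projectile Blueprint fired by enemies, with its launch handled in OnSpawn.
; OnSpawn scales the actor's current velocity by a Speed argument, adds random per-axis jitter for spread, and writes the result to ProjectileMovement.
; It plays the shot sound at the root's location, then destroys itself after a Lifetime delay.
; The construction script only calls the parent's, and the graph contains no hit or damage logic.
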(event `OnSpawn`
  (params (Speed :type "Float (double-precision)"))
  (bind (_returnvalue_x _returnvalue_y _returnvalue_z) (`KismetMathLibrary.BreakVector` (* (`self.GetVelocity`) Speed)))
  (set `MovementComponent.Velocity` (`KismetMathLibrary.MakeVector` (+ (`KismetMathLibrary.RandomFloatInRange` -100.0 100.0) _returnvalue_x) (+ (`KismetMathLibrary.RandomFloatInRange` -100.0 100.0) _returnvalue_y) (+ (`KismetMathLibrary.RandomFloatInRange` -100.0 100.0) _returnvalue_z)) (`self.ProjectileMovement`))
  (`GameplayStatics.PlaySoundAtLocation` "/Game/Assets/Sound/shot.shot" (`SceneComponent.K2_GetComponentLocation` (`self.DefaultSceneRoot`)) (struct) 1.0 1.0 0.0 null null null null)
  (`KismetSystemLibrary.Delay` (`self.Lifetime`))
  (`self.K2_DestroyActor`))

(fn `UserConstructionScript`
  (`parent.UserConstructionScript`))
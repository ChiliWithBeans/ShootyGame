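; BP_Enemy_Turret is an enemy turret that aims at the player, can fire ball projectiles and is destroyed when its health runs out.
; PawnSensing stores the player on first sight and never clears that state.
; Tick lerps the turret toward the player, faster at short range.
; While IsShooting, which this graph never sets, it spawns projectiles on a Delay-gated cooldown, with speed scaled by clamped distance.
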(event `self.ReceiveTick`
  (params (DeltaSeconds :type "Float (single-precision)"))
  (bind (_returnvalue_location _returnvalue_rotation) (`KismetMathLibrary.BreakTransform` (`SceneComponent.K2_GetComponentToWorld` (`self.turret`))))
  (bind _returnvalue (`self.K2_GetActorLocation` (`self.PlayerRef`)))
  (if (`self.SeesPlayer`)
    ;[1 1 1] Used to determine projectile speed
    (set `self.PlayerDistance` (`KismetMathLibrary.VSize` (- _returnvalue_location _returnvalue)))
    (set `self.RotationSpeed` (`KismetMathLibrary.FClamp` (- 1.0 (/ (`self.PlayerDistance`) 2000.0)) 0.05 1.0))
    (`SceneComponent.K2_SetWorldRotation` (`self.turret`) (`KismetMathLibrary.RLerp` _returnvalue_rotation (`KismetMathLibrary.FindLookAtRotation` _returnvalue_location _returnvalue) (`self.RotationSpeed`) (`self.IsShooting`)) false false)
    (if (and (`self.IsShooting`) (`self.ShootingDelayPassed`))
      (bind _returnvalue_2 (`|SpawnActorFromClass` "/Game/Assets/Blueprints/Enemies/BP_EnemyProjectile_Ball.BP_EnemyProjectile_Ball_C" (`SceneComponent.K2_GetComponentToWorld` (`self.ProjectileSpawnPoint`)) "Undefined" "OverrideRootScale" null null))
      (`/Engine/EditorBlueprintResources/StandardMacros.IsValid` _returnvalue_2
        (:`Is Valid`
          ;[1 1 1] Projectile speed increases with distance from target
          (`/Game/Assets/Blueprints/Enemies/BP_EnemyProjectile_Ball.OnSpawn` _returnvalue_2 (`KismetMathLibrary.FClamp` (`self.PlayerDistance`) 3000.0 10000.0)))
        (:`Is Not Valid`
          _))
      (set `self.ShootingDelayPassed` false)
      (`KismetSystemLibrary.Delay` (`self.FireDelay`))
      (set `self.ShootingDelayPassed` true))))

(event `self.PawnSensing.OnSeePawn`
  (params (Pawn :type "Pawn Object Reference"))
  (bind _asbp_player_character (cast `/Game/Assets/Blueprints/BP_PlayerCharacter` Pawn))
  (set `self.PlayerRef` _asbp_player_character)
  (set `self.SeesPlayer` true))

(event `self.Take Damage`
  (params (Amount :type "Float (double-precision)"))
  ;[1 1 1] Triggered by projectiles hitting this actor
  (bind _output_get (set `self.Health` (- (`self.Health`) Amount)))
  (if (<= _output_get 0.0)
    (`self.K2_DestroyActor`)))

(fn `UserConstructionScript`
  (`parent.UserConstructionScript`))
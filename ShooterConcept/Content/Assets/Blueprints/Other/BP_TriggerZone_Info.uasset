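; BP_TriggerZone_Info is a one-shot trigger zone that tells the player they found secret protein powder.
; When an enabled zone is overlapped by BP_PlayerCharacter, it writes a hard-coded message to that character's InfoBoxRef and disables itself to block retriggers.
; After a short delay it clears the text and destroys itself.
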(event `self.ReceiveActorBeginOverlap`
  (params (OtherActor :type "Actor Object Reference"))
  (if (`self.Enabled`)
    (bind _asbp_player_character (cast `/Game/Assets/Blueprints/BP_PlayerCharacter` OtherActor))
    (bind _infobox_ref (`/Game/Assets/Blueprints/BP_PlayerCharacter.InfoBox Ref` _asbp_player_character))
    (`/Game/Assets/Blueprints/UI/BP_UI_Info.Update Text` _infobox_ref "Secret Protein Powder Found!")
    (set `self.Enabled` false)
    (`KismetSystemLibrary.Delay` 5.0)
    (`/Game/Assets/Blueprints/UI/BP_UI_Info.Update Text` _infobox_ref "")
    (`self.K2_DestroyActor`)))

(fn `UserConstructionScript`
  (`parent.UserConstructionScript`))
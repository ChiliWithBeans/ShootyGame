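; Player character Blueprint for a shooter, with movement, camera look, two weapon slots and battle rifle pickups.
; Each tick, a screen-center trace records the looked-at actor for interaction and rotates the equipped weapon toward the aim point.
; Mouse wheel swapping toggles two Child Actor components holding rifle or pistol.
; Fire, reload, drop and special-action inputs only reach a battle rifle in the first slot, whichever is equipped.
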(event `self.ReceiveTick`
  (params (DeltaSeconds :type "Float (single-precision)"))
  (bind _returnvalue (`GameplayStatics.GetPlayerController` 0))
  (bind _returnvalue_2 (`SceneComponent.K2_GetComponentRotation` (`self.Camera`)))
  (bind (_sizex _sizey) (`PlayerController.GetViewportSize` _returnvalue))
  (bind (_worldposition _worlddirection) (`GameplayStatics.DeprojectScreenToWorld` _returnvalue (`KismetMathLibrary.MakeVector2D` (`KismetMathLibrary.Conv_IntToDouble` (/ _sizex 2)) (`KismetMathLibrary.Conv_IntToDouble` (/ _sizey 2)))))
  ;[1 1 1] Aim Weapon Towards Crosshair
  (bind _outhit (`KismetSystemLibrary.LineTraceSingle` :`Start` _worldposition :`End` (+ (* _worlddirection (`KismetMathLibrary.Conv_DoubleToVector` 10000.0)) _worldposition) :`TraceChannel` "TraceTypeQuery1" :`DrawDebugType` "ForOneFrame"))
  (set `self.LookedAtObject` (`.HitActor` (`GameplayStatics.BreakHitResult` _outhit)))
  (set `self.AimPointDistance` (`.Distance` (`GameplayStatics.BreakHitResult` _outhit)))
  (if (== (`.Location` (`GameplayStatics.BreakHitResult` _outhit)) (0.0 0.0 0.0))
    (switch `int` (`self.EquippedWeaponSlot`)
      (:`0`
        (bind _asbp_battle_rifle (cast `/Game/Assets/Blueprints/BP_BattleRifle` (`ChildActorComponent.ChildActor` (`self.Weapon`))))
        (`/Game/Assets/Blueprints/BP_BattleRifle.WeaponRotation` _asbp_battle_rifle (`.Location` (`GameplayStatics.BreakHitResult` _outhit)) false _returnvalue_2)
        (`/Game/Assets/Blueprints/BP_BattleRifle.WeaponFunction` _asbp_battle_rifle (`self.BattleRifleUI`)))
      (:`1`
        (bind _asbp_pistol (cast `/Game/Assets/Blueprints/BP_Pistol` (`ChildActorComponent.ChildActor` (`self.Weapon2`))))
        (`/Game/Assets/Blueprints/BP_Pistol.WeaponRotation` _asbp_pistol (`.Location` (`GameplayStatics.BreakHitResult` _outhit)) false (`SceneComponent.K2_GetComponentRotation` (`self.Camera`)))))
    (else
      (switch `int` (`self.EquippedWeaponSlot`)
        (:`0`
          (bind _asbp_battle_rifle_2 (cast `/Game/Assets/Blueprints/BP_BattleRifle` (`ChildActorComponent.ChildActor` (`self.Weapon`))))
          (`/Game/Assets/Blueprints/BP_BattleRifle.WeaponRotation` _asbp_battle_rifle_2 (`.Location` (`GameplayStatics.BreakHitResult` _outhit)) true _returnvalue_2)
          (`/Game/Assets/Blueprints/BP_BattleRifle.WeaponFunction` _asbp_battle_rifle_2 (`self.BattleRifleUI`)))
        (:`1`
          (bind _asbp_pistol_2 (cast `/Game/Assets/Blueprints/BP_Pistol` (`ChildActorComponent.ChildActor` (`self.Weapon2`))))
          (`/Game/Assets/Blueprints/BP_Pistol.WeaponRotation` _asbp_pistol_2 (`.Location` (`GameplayStatics.BreakHitResult` _outhit)) true (`SceneComponent.K2_GetComponentRotation` (`self.Camera`))))))))

(event `self.ReceiveBeginPlay`
  (set `self.Weapon0` "NewEnumerator0")
  (set `self.Weapon1` "NewEnumerator1")
  (bind _returnvalue (`|CreateWidget` "/Game/Assets/Blueprints/BP_UI_BR.BP_UI_BR_C" (`GameplayStatics.GetPlayerController` 0)))
  (bind _output_get (set `self.BattleRifleUI` _returnvalue))
  (`UserWidget.AddToViewport` _output_get 0)
  (`ChildActorComponent.SetChildActorClass` (`self.Weapon`) "/Game/Assets/Blueprints/BP_BattleRifle.BP_BattleRifle_C")
  (`ChildActorComponent.SetChildActorClass` (`self.Weapon2`) "/Game/Assets/Blueprints/BP_Pistol.BP_Pistol_C")
  (`self.WeaponSwap` (`self.EquippedWeaponSlot`)))

(event `InputAxis|ForwardBack`
  (params (AxisValue :type "Float (single-precision)"))
  (bind (_returnvalue_roll _returnvalue_pitch _returnvalue_yaw) (`KismetMathLibrary.BreakRotator` (`SceneComponent.K2_GetComponentRotation` (`self.Camera`))))
  ;[1 1 1] Forward/Back movement
  (`self.AddMovementInput` (`KismetMathLibrary.GetForwardVector` (`KismetMathLibrary.MakeRotator` 0.0 0.0 _returnvalue_yaw)) AxisValue))

(event `InputAxis|RightLeft`
  (params (AxisValue :type "Float (single-precision)"))
  (bind (_returnvalue_roll _returnvalue_pitch _returnvalue_yaw) (`KismetMathLibrary.BreakRotator` (`SceneComponent.K2_GetComponentRotation` (`self.Camera`))))
  ;[1 1 1] Right/Left movement
  (`self.AddMovementInput` (`KismetMathLibrary.GetRightVector` (`KismetMathLibrary.MakeRotator` 0.0 0.0 _returnvalue_yaw)) AxisValue))

(event `InputAction|Jump`
  (params (Key :type "Key Structure"))
  ;[1 1 1] Inputs
  (:`Pressed`
    (`self.Jump`)))

(event `InputAction|Main`
  (params (Key :type "Key Structure"))
  ;[1 1 1] Inputs
  (:`Pressed`
    (bind _asbp_battle_rifle (cast `/Game/Assets/Blueprints/BP_BattleRifle` (`ChildActorComponent.ChildActor` (`self.Weapon`)))
      (:`then`
        (`/Game/Assets/Blueprints/BP_BattleRifle.StartFiring` _asbp_battle_rifle))
      (:`CastFailed`
        (`KismetSystemLibrary.PrintString` "no weapon"))))
  (:`Released`
    (bind _asbp_battle_rifle_2 (cast `/Game/Assets/Blueprints/BP_BattleRifle` (`ChildActorComponent.ChildActor` (`self.Weapon`))))
    (`/Game/Assets/Blueprints/BP_BattleRifle.StopFiring` _asbp_battle_rifle_2)))

(event `InputAxis|MouseWheel`
  (params (AxisValue :type "Float (single-precision)"))
  (bind _maxweaponslot (`self.MaxWeaponSlot`))
  (bind _returnvalue (+ (`KismetMathLibrary.Round` AxisValue) (`self.EquippedWeaponSlot`)))
  ;[1 1 1] Weapon Swap
  ;;[1 1 1] Change equipped weapon with mouse wheel
  (if (!= AxisValue 0.0)
    (if (>= _returnvalue 0)
      (if (> _returnvalue _maxweaponslot)
        (bind _output_get (set `self.EquippedWeaponSlot` 0))
        (`self.WeaponSwap` _output_get)
        (else
          (bind _output_get_2 (set `self.EquippedWeaponSlot` _returnvalue))
          (`self.WeaponSwap` _output_get_2)))
      (else
        (bind _output_get_3 (set `self.EquippedWeaponSlot` _maxweaponslot))
        (`self.WeaponSwap` _output_get_3)))))

(event `InputAxis|Pitch`
  (params (AxisValue :type "Float (single-precision)"))
  (bind _camera (`self.Camera`))
  (bind (_returnvalue_roll _returnvalue_pitch _returnvalue_yaw) (`KismetMathLibrary.BreakRotator` (`SceneComponent.K2_GetComponentRotation` _camera)))
  (bind (_returnvalue_roll_2 _returnvalue_pitch_2) (`KismetMathLibrary.BreakRotator` (`SceneComponent.K2_GetComponentRotation` _camera)))
  ;[1 1 1] Camera Rotation
  (`SceneComponent.K2_SetWorldRotation` _camera (`KismetMathLibrary.MakeRotator` 0.0 (`KismetMathLibrary.FClamp` (+ _returnvalue_pitch_2 AxisValue) -85.0 85.0) (+ _returnvalue_yaw (stale `InputAxis|Yaw` AxisValue))) false false :!label _label))

(event `InputAction|Crouch`
  (params (Key :type "Key Structure"))
  ;[1 1 1] Inputs
  (:`Pressed`
    (`self.Crouch`))
  (:`Released`
    (`self.UnCrouch`)))

(event `InputAction|Action 2`
  (params (Key :type "Key Structure"))
  ;[1 1 1] Inputs
  (:`Pressed`
    (bind _asbp_battle_rifle (cast `/Game/Assets/Blueprints/BP_BattleRifle` (`ChildActorComponent.ChildActor` (`self.Weapon`))))
    (`/Game/Assets/Blueprints/BP_BattleRifle.Railgun` _asbp_battle_rifle)))

(event `InputAxis|Yaw`
  (params (AxisValue :type "Float (single-precision)"))
  ;[1 1 1] Camera Rotation
  (goto _label))

(event `InputAction|Secondary`
  (params (Key :type "Key Structure"))
  ;[1 1 1] Inputs
  (:`Pressed`
    (bind _asbp_battle_rifle (cast `/Game/Assets/Blueprints/BP_BattleRifle` (`ChildActorComponent.ChildActor` (`self.Weapon`))))
    (`/Game/Assets/Blueprints/BP_BattleRifle.ActiveCoolingStart` _asbp_battle_rifle))
  (:`Released`
    (bind _asbp_battle_rifle_2 (cast `/Game/Assets/Blueprints/BP_BattleRifle` (`ChildActorComponent.ChildActor` (`self.Weapon`))))
    (`/Game/Assets/Blueprints/BP_BattleRifle.ActiveCoolingStop` _asbp_battle_rifle_2)))

(event `InputAction|Action 3`
  (params (Key :type "Key Structure"))
  ;[1 1 1] Inputs
  (:`Pressed`
    (bind _asbp_battle_rifle (cast `/Game/Assets/Blueprints/BP_BattleRifle` (`ChildActorComponent.ChildActor` (`self.Weapon`))))
    (`/Game/Assets/Blueprints/BP_BattleRifle.BarrelChange` _asbp_battle_rifle)))

(event `WeaponSwap`
  (params (EquippedWeaponSlot :type Integer))
  (bind _weapon (`self.Weapon`))
  (bind _weapon2 (`self.Weapon2`))
  (bind _weapon_2 (`self.Weapon`))
  (bind _weapon2_2 (`self.Weapon2`))
  ;[1 1 1] Weapon Swap
  (switch `int` EquippedWeaponSlot
    (:`0`
      (`ActorComponent.SetActive` _weapon_2 true false)
      (`SceneComponent.SetHiddenInGame` _weapon_2 false true)
      (`ActorComponent.Deactivate` _weapon2)
      (`SceneComponent.SetHiddenInGame` _weapon2 true true))
    (:`1`
      (`ActorComponent.SetActive` _weapon2_2 true false)
      (`SceneComponent.SetHiddenInGame` _weapon2_2 false true)
      (`ActorComponent.Deactivate` _weapon)
      (`SceneComponent.SetHiddenInGame` _weapon true true))))

(event `InputAction|Action 1`
  (params (Key :type "Key Structure"))
  ;[1 1 1] Inputs
  (:`Pressed`
    (bind _asbp_battle_rifle (cast `/Game/Assets/Blueprints/BP_BattleRifle` (`ChildActorComponent.ChildActor` (`self.Weapon`))))
    (`/Game/Assets/Blueprints/BP_BattleRifle.Stabilizer` _asbp_battle_rifle)))

(event `InputAction|Reload`
  (params (Key :type "Key Structure"))
  ;[1 1 1] Inputs
  ;;[1 1 1] Reload
  (:`Released`
    (bind _asbp_battle_rifle (cast `/Game/Assets/Blueprints/BP_BattleRifle` (`ChildActorComponent.ChildActor` (`self.Weapon`))))
    (`/Game/Assets/Blueprints/BP_BattleRifle.Reload` _asbp_battle_rifle)))

(event `InputAction|Interact`
  (params (Key :type "Key Structure"))
  ;[1 1 1] Inputs
  ;;[1 1 1] Interaction, currently only used to pick up weapons
  (:`Pressed`
    (if (<= (`self.AimPointDistance`) (`self.InteractionRange`))
      (bind _asbp_weapon_drop_br (cast `/Game/Assets/Blueprints/BP_WeaponDropBR` (`self.LookedAtObject`)))
      (`/Game/Assets/Blueprints/BP_WeaponDropBR.WeaponPickup` _asbp_weapon_drop_br self))))

(event `InputAction|TestAction1`
  (params (Key :type "Key Structure"))
  ;[1 1 1] Inputs
  (:`Pressed`
    (bind _asbp_battle_rifle (cast `/Game/Assets/Blueprints/BP_BattleRifle` (`ChildActorComponent.ChildActor` (`self.Weapon`))))
    (`/Game/Assets/Blueprints/BP_BattleRifle.WeaponDrop` _asbp_battle_rifle (`SceneComponent.GetForwardVector` (`self.Camera`)))))

(event `InputAction|TestAction2`
  (params (Key :type "Key Structure"))
  ;[1 1 1] Inputs
)

(event `WeaponPickupBR`
  (params (Magazines :type Integer) (Ammo :type Integer) (Charge :type "Float (double-precision)") (`Heat Active` :type "Float (double-precision)") (`Heat Spare` :type "Float (double-precision)"))
  ;[1 1 1] Weapon Pickups
  (switch `int` (`self.EquippedWeaponSlot`)
    (:`0`
      (set `self.Weapon0` "NewEnumerator0")
      (`ChildActorComponent.SetChildActorClass` (`self.Weapon`) "/Game/Assets/Blueprints/BP_BattleRifle.BP_BattleRifle_C")
      (bind _asbp_battle_rifle (cast `/Game/Assets/Blueprints/BP_BattleRifle` (`ChildActorComponent.ChildActor` (`self.Weapon`))))
      (`/Game/Assets/Blueprints/BP_BattleRifle.OnPickedUp` _asbp_battle_rifle Magazines Ammo Charge `Heat Active` `Heat Spare`))
    (:`1`
      (set `self.Weapon1` "NewEnumerator0")
      (`ChildActorComponent.SetChildActorClass` (`self.Weapon2`) "/Game/Assets/Blueprints/BP_BattleRifle.BP_BattleRifle_C")
      (bind _asbp_battle_rifle_2 (cast `/Game/Assets/Blueprints/BP_BattleRifle` (`ChildActorComponent.ChildActor` (`self.Weapon2`))))
      (`/Game/Assets/Blueprints/BP_BattleRifle.OnPickedUp` _asbp_battle_rifle_2 Magazines Ammo Charge `Heat Active` `Heat Spare`))))

(fn `UserConstructionScript`)
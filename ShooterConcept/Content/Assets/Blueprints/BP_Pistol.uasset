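; Pistol actor Blueprint that animates the weapon's rotation and position to follow the aim, with no firing logic in this file.
; The WeaponRotation event turns the pistol toward the aim point, or to the camera rotation when none exists.
; An aim point within a short distance of the root counts as an obstacle, pitching the pistol up and pulling it back.
; Frame-time-based RInterpTo and VInterpTo smooth both motions at AnimationSpeed.
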(event `WeaponRotation`
  (params (AimPoint :type "Vector Structure") (DoesAimPointExist :type Boolean) (CameraRotation :type "Rotator Structure"))
  (bind _returnvalue (`SceneComponent.K2_GetComponentRotation` (`self.Pistol`)))
  ;[1 1 1] Weapon Rotation
  (set `self.IsThereNoObstacle` (> (`KismetMathLibrary.VSize` (- (`SceneComponent.K2_GetComponentLocation` (`self.DefaultSceneRoot`)) AimPoint)) 40.0))
  (if DoesAimPointExist
    (if (`self.IsThereNoObstacle`)
      (`SceneComponent.K2_SetWorldRotation` (`self.Pistol`) (`KismetMathLibrary.RInterpTo` _returnvalue (`KismetMathLibrary.FindLookAtRotation` (`SceneComponent.K2_GetComponentLocation` (`self.Pistol`)) AimPoint) (`GameplayStatics.GetWorldDeltaSeconds`) (`self.Animation Speed`)) false false)
      (else
        (`SceneComponent.K2_SetWorldRotation` (`self.Pistol`) (`KismetMathLibrary.RInterpTo` _returnvalue (`KismetMathLibrary.MakeRotator` (.roll CameraRotation) (`KismetMathLibrary.FClamp` (+ (.pitch CameraRotation) 85.0) -85.0 85.0) (.yaw CameraRotation)) (`GameplayStatics.GetWorldDeltaSeconds`) (`self.Animation Speed`)) false false)))
    (else
      (`SceneComponent.K2_SetWorldRotation` (`self.Pistol`) (`KismetMathLibrary.RInterpTo` _returnvalue CameraRotation (`GameplayStatics.GetWorldDeltaSeconds`) (`self.Animation Speed`)) false false)))
  (if (`self.IsThereNoObstacle`)
    (`SceneComponent.K2_SetRelativeLocation` (`self.Pistol`) (`KismetMathLibrary.VInterpTo` (`SceneComponent.RelativeLocation` (`self.Pistol`)) (0.0 0.0 0.0) (`GameplayStatics.GetWorldDeltaSeconds`) (`self.Animation Speed`)) false false)
    (else
      (`SceneComponent.K2_SetRelativeLocation` (`self.Pistol`) (`KismetMathLibrary.VInterpTo` (`SceneComponent.RelativeLocation` (`self.Pistol`)) (-50.0 0.0 20.0) (`GameplayStatics.GetWorldDeltaSeconds`) (`self.Animation Speed`)) false false))))

(fn `UserConstructionScript`)